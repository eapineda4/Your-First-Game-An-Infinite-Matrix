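; BP_HealthPack is a health pickup actor that heals the player by removing one recorded hit.
; On a Hit event it disables its Cube's collision, then lowers BP_Player's Hits counter if non-zero and refreshes the HealthBar.
; It always targets player pawn 0 without checking what hit it, and it neither hides nor destroys itself.
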(event `self.ReceiveHit`
  (params (MyComp :type "PrimitiveComponent Object Reference") (Other :type "Actor Object Reference") (OtherComp :type "PrimitiveComponent Object Reference") (bSelfMoved :type Boolean) (HitLocation :type "Vector Structure") (HitNormal :type "Vector Structure") (NormalImpulse :type "Vector Structure") (Hit :type "HitResult Structure (by ref)"))
  (`PrimitiveComponent.SetCollisionEnabled` (`self.Cube`) "NoCollision")
  (bind _asbp_player (cast `/Game/InfiniteMatrix/Blueprints/BP_Player` (`GameplayStatics.GetPlayerPawn` 0)))
  (bind _hits (`/Game/InfiniteMatrix/Blueprints/BP_Player.Hits` _asbp_player))
  (if (!= 0.0 _hits)
    (set `/Game/InfiniteMatrix/Blueprints/BP_Player.Hits` (- _hits 1.0) _asbp_player)
    (`/Game/InfiniteMatrix/Blueprints/UI_HealthBar.Update Health Bar` (`/Game/InfiniteMatrix/Blueprints/BP_Player.Health Bar` _asbp_player))))

(fn `UserConstructionScript`)