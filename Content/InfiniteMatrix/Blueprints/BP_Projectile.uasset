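; BP_Projectile is a shot that destroys any BP_Enemy it hits and has the player's BP_Player pawn update the score.
; Hitting anything else simply destroys the projectile.
; Every Tick, SetSpeed sets the ProjectileMovement component's initial and max speed to a fixed multiple of the player's ForwardSpeed.
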(event `self.ReceiveBeginPlay`)

(event `self.ReceiveTick`
  (params (DeltaSeconds :type "Float (single-precision)"))
  (`self.SetSpeed`))

(event `self.ReceiveHit`
  (params (MyComp :type "PrimitiveComponent Object Reference") (Other :type "Actor Object Reference") (OtherComp :type "PrimitiveComponent Object Reference") (bSelfMoved :type Boolean) (HitLocation :type "Vector Structure") (HitNormal :type "Vector Structure") (NormalImpulse :type "Vector Structure") (Hit :type "HitResult Structure (by ref)"))
  (bind _asbp_enemy (cast `/Game/InfiniteMatrix/Blueprints/BP_Enemy` Other)
    (:`then`
      (`self.K2_DestroyActor` _asbp_enemy)
      (bind _asbp_player (cast `/Game/InfiniteMatrix/Blueprints/BP_Player` (`GameplayStatics.GetPlayerPawn` 0)))
      (`/Game/InfiniteMatrix/Blueprints/BP_Player.Update Score` _asbp_player))
    (:`CastFailed`
      _))
  (`self.K2_DestroyActor`))

(fn `SetSpeed`
  (bind _projectilemovement (`self.ProjectileMovement`))
  (bind _asbp_player (cast `/Game/InfiniteMatrix/Blueprints/BP_Player` (`GameplayStatics.GetPlayerPawn` 0)))
  (bind _returnvalue (* 3.0 (`/Game/InfiniteMatrix/Blueprints/BP_Player.ForwardSpeed` _asbp_player)))
  (set `ProjectileMovementComponent.MaxSpeed` _returnvalue _projectilemovement)
  (set `ProjectileMovementComponent.InitialSpeed` _returnvalue _projectilemovement))

(fn `UserConstructionScript`)