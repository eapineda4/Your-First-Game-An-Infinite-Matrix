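; Tunnel segment of an endless obstacle run, with a rotating holed wall that registers hits on BP_Player.
; On BeginPlay it always spawns an enemy, sometimes a health pack, and picks tunnel and wall materials by score tier.
; Crossing TriggerZone has TunnelSpawner add a segment, destroys this one and updates score; wall hits disable its collision unless the player is dead.
; RandomizeWall picks a random hole mesh and roll, but is not called here.
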(event `self.ReceiveBeginPlay`
  (bind _staticmeshcomponent (`self.StaticMeshComponent`))
  (bind _wallmesh (`self.WallMesh`))
  (`self.SpawnHealthPack`)
  (`self.SpawnEnemy`)
  (bind _asbp_player (cast `/Game/InfiniteMatrix/Blueprints/BP_Player` (`GameplayStatics.GetPlayerPawn` 0)))
  (bind _score (`/Game/InfiniteMatrix/Blueprints/BP_Player.Score` _asbp_player))
  (if (>= _score 15.0)
    (if (>= _score 25.0)
      (if (>= _score 35.0)
        (if (>= _score 50.0)
          (`PrimitiveComponent.SetMaterial` _staticmeshcomponent 0 "/Game/InfiniteMatrix/Materials/MI_Tunnel_v4.MI_Tunnel_v4")
          (`PrimitiveComponent.SetMaterial` _wallmesh 0 "/Game/InfiniteMatrix/Materials/MI_Holev4.MI_Holev4")
          (else
            (`PrimitiveComponent.SetMaterial` _staticmeshcomponent 0 "/Game/InfiniteMatrix/Materials/MI_Tunnel_v3.MI_Tunnel_v3" :!label _label)
            (`PrimitiveComponent.SetMaterial` _wallmesh 0 "/Game/InfiniteMatrix/Materials/MI_Holev3.MI_Holev3")))
        (else
          (goto _label)))
      (else
        (`PrimitiveComponent.SetMaterial` _staticmeshcomponent 0 "/Game/InfiniteMatrix/Materials/MI_Tunnel_v2.MI_Tunnel_v2")
        (`PrimitiveComponent.SetMaterial` _wallmesh 0 "/Game/InfiniteMatrix/Materials/MI_Holev2.MI_Holev2")))))

(event `self.ReceiveTick`
  (params (DeltaSeconds :type "Float (single-precision)"))
  (`SceneComponent.K2_AddLocalRotation` (`self.WallMesh`) (`KismetMathLibrary.MakeRotator` (* DeltaSeconds (`self.RotateSpeed`))) false false))

(event `self.TriggerZone.OnComponentBeginOverlap`
  (params (OverlappedComponent :type "PrimitiveComponent Object Reference") (OtherActor :type "Actor Object Reference") (OtherComp :type "PrimitiveComponent Object Reference") (OtherBodyIndex :type Integer) (bFromSweep :type Boolean) (SweepResult :type "HitResult Structure (by ref)"))
  (bind _asbp_player (cast `/Game/InfiniteMatrix/Blueprints/BP_Player` OtherActor))
  (`/Game/InfiniteMatrix/Blueprints/BP_TunnelSpawner.SpawnTunnelAtSpawnPoint` (`self.TunnelSpawner`))
  (`self.K2_DestroyActor`)
  (`/Game/InfiniteMatrix/Blueprints/BP_Player.Update Score` _asbp_player))

(event `self.WallMesh.OnComponentHit`
  (params (HitComponent :type "PrimitiveComponent Object Reference") (OtherActor :type "Actor Object Reference") (OtherComp :type "PrimitiveComponent Object Reference") (NormalImpulse :type "Vector Structure") (Hit :type "HitResult Structure (by ref)"))
  (bind _asbp_player (cast `/Game/InfiniteMatrix/Blueprints/BP_Player` OtherActor))
  (`/Game/InfiniteMatrix/Blueprints/BP_Player.Count Hits` _asbp_player)
  (if (not (`/Game/InfiniteMatrix/Blueprints/BP_Player.IsDead` _asbp_player))
    (`PrimitiveComponent.SetCollisionEnabled` (`self.WallMesh`) "NoCollision")))

(fn `RandomizeWall`
  (`StaticMeshComponent.SetStaticMesh` (`self.WallMesh`) (select `int` (`KismetMathLibrary.RandomIntegerInRange` 0 3) :`0` "/Game/InfiniteMatrix/Meshes/SM_Hole_01.SM_Hole_01" :`1` "/Game/InfiniteMatrix/Meshes/SM_Hole_02.SM_Hole_02" :`2` "/Game/InfiniteMatrix/Meshes/SM_Hole_03.SM_Hole_03" :`3` "/Game/InfiniteMatrix/Meshes/SM_Hole_04.SM_Hole_04" :!type "StaticMesh Object Reference"))
  (`SceneComponent.K2_AddLocalRotation` (`self.WallMesh`) (`KismetMathLibrary.MakeRotator` (`KismetMathLibrary.RandomFloatInRange` 0.0 360.0)) false false))

(fn `SpawnEnemy`
  (bind _returnvalue (`KismetMathLibrary.RandomFloatInRange` 0.0 300.0))
  (bind _returnvalue_2 (`KismetMathLibrary.RandomFloatInRange` -1150.0 1150.0))
  (if (== (`KismetMathLibrary.RandomInteger` 1) 0)
    (`|SpawnActorFromClass` "/Game/InfiniteMatrix/Blueprints/BP_Enemy.BP_Enemy_C" (`KismetMathLibrary.MakeTransform` (+ (`SceneComponent.K2_GetComponentLocation` (`self.HealthSpawnZone`)) (`KismetMathLibrary.MakeVector` (`KismetMathLibrary.RandomFloatInRange` 0.0 350.0) (* _returnvalue_2 (`KismetMathLibrary.DegCos` _returnvalue)) (* _returnvalue_2 (`KismetMathLibrary.DegSin` _returnvalue)))) (struct) (1.5 1.5 1.5)) "Undefined" "MultiplyWithRoot" null null)))

(fn `SpawnHealthPack`
  (bind _returnvalue (`KismetMathLibrary.RandomFloatInRange` 0.0 360.0))
  (bind _returnvalue_2 (`KismetMathLibrary.RandomFloatInRange` -1200.0 1200.0))
  (if (== (`KismetMathLibrary.RandomInteger` 3) 0)
    (`|SpawnActorFromClass` "/Game/InfiniteMatrix/Blueprints/BP_HealthPack.BP_HealthPack_C" (`KismetMathLibrary.MakeTransform` (+ (`SceneComponent.K2_GetComponentLocation` (`self.HealthSpawnZone`)) (`KismetMathLibrary.MakeVector` (`KismetMathLibrary.RandomFloatInRange` 0.0 390.0) (* _returnvalue_2 (`KismetMathLibrary.DegCos` _returnvalue)) (* _returnvalue_2 (`KismetMathLibrary.DegSin` _returnvalue)))) (struct) (0.8 0.8 0.8)) "Undefined" "MultiplyWithRoot" null null)))

(fn `UserConstructionScript`)